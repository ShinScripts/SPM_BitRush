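; BP_EnemyRocketTurret is an enemy turret that tracks the player pawn and periodically shoots.
; On Tick, while the player is within range, it snaps the whole actor's rotation to face them.
; The same Tick chain runs a Delay before calling Shoot, so the latent node's ignored retriggers act as the fire-rate throttle.
; Shoot is called here but defined outside these graphs.
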(event `self.ReceiveTick`
  (params (DeltaSeconds :type "Float (single-precision)"))
  (bind _returnvalue (- (`self.K2_GetActorLocation` (`GameplayStatics.GetPlayerPawn` 0)) (`self.K2_GetActorLocation`)))
  (if (< (`KismetMathLibrary.Vector_Distance` _returnvalue) 10000.0)
    (`self.K2_SetActorRotation` (`KismetMathLibrary.Conv_VectorToRotator` _returnvalue))
    (`KismetSystemLibrary.Delay` 7.0)
    (`self.Shoot`)))

(fn `UserConstructionScript`)