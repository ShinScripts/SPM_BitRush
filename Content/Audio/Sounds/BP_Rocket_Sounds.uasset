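; Component that handles the sounds of a rocket projectile: flight, approach and destruction.
; BeginPlay attaches the flight cue to the owner's mesh, and Tick attaches a one-shot closing-in sound to that audio once the player is within range.
; EndPlay sets a short owner lifespan and plays a destruction sound with randomized volume and pitch, plus an angry robot sound if the owner overlaps the player.
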(event `self.ReceiveBeginPlay`
  (bind _returnvalue (`GameplayStatics.SpawnSoundAttached` "/Game/Audio/Sounds/Unsorted/PH_RocketProjectile_Flight_Cue.PH_RocketProjectile_Flight_Cue" (`Actor.GetComponentByClass` (`self.GetOwner`) "/Script/Engine.MeshComponent") "None" (0.0 0.0 0.0) (struct) "KeepRelativeOffset" true 1.0 1.0 0.0 null null)))

(event `self.ReceiveTick`
  (params (DeltaSeconds :type "Float (single-precision)"))
  (if (< (`KismetMathLibrary.Vector_Distance` (`Actor.K2_GetActorLocation` (`self.GetOwner`)) (`Actor.K2_GetActorLocation` (`GameplayStatics.GetPlayerCharacter` 0))) 400.0)
    (`/Engine/EditorBlueprintResources/StandardMacros.DoOnce` false
      (:`Completed`
        (`GameplayStatics.SpawnSoundAttached` "/Game/Audio/Sounds/Unsorted/PH_RocketClosingIn.PH_RocketClosingIn" (stale `self.ReceiveBeginPlay` _returnvalue) "None" (0.0 0.0 0.0) (struct) "KeepRelativeOffset" true 1.0 1.0 0.0 "/Game/Audio/RocketClosingAttenuation.RocketClosingAttenuation" null)))))

(event `self.ReceiveEndPlay`
  (params (EndPlayReason :type "EEndPlayReason Enum" :default "Destroyed"))
  (bind _returnvalue (`KismetMathLibrary.RandomFloatInRange` 0.8 1.1))
  (`Actor.SetLifeSpan` (`self.GetOwner`) 0.2)
  (`GameplayStatics.PlaySoundAtLocation` "/Game/Audio/Sounds/MSS_Destruction_Sounds.MSS_Destruction_Sounds" (0.0 0.0 0.0) (struct) _returnvalue _returnvalue 0.0 null null null null)
  (if (`Actor.IsOverlappingActor` (`self.GetOwner`) (`GameplayStatics.GetPlayerCharacter` 0))
    (`GameplayStatics.PlaySoundAtLocation` "/Game/Audio/Sounds/Vocalizations/PH_Angry_Robot2.PH_Angry_Robot2" (0.0 0.0 0.0) (struct) 0.4 1.0 0.0 null null null null)))

(fn `NewFunction`)