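; Player audio Blueprint that plays one-shot movement and action sounds, with randomized volume and pitch, for the player character cached at BeginPlay.
; Input events trigger jump, slide, dash (gated by CanDash) and left-click fire sounds.
; Tick polls player state through DoOnce latches: CanGrapple plays a drone, Landed re-arms the jump sound, and camera roll past a threshold stands in for wall-run detection.
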(event `self.ReceiveBeginPlay`
  ;[1 1 1] Get Player Reference
  (bind _asbp_player_character (cast `/Game/Blueprints/BP_PlayerCharacter` (`GameplayStatics.GetPlayerCharacter` 0)))
  (set `self.Player` _asbp_player_character))

(event `InputAction|Jump` :consume false
  (params (Key :type "Key Structure"))
  (bind _returnvalue (`KismetMathLibrary.RandomFloatInRange` 0.95 1.05))
  (:`Pressed`
    (`/Engine/EditorBlueprintResources/StandardMacros.DoOnce` false :!label _label
      (:`Completed`
        (`GameplayStatics.PlaySoundAtLocation` "/Game/Audio/Sounds/MSS_Jump_Sounds.MSS_Jump_Sounds" (`self.K2_GetActorLocation` (`self.Player`)) (struct) _returnvalue _returnvalue 0.0 null null null null)))))

(event `self.ReceiveTick`
  (params (DeltaSeconds :type "Float (single-precision)"))
  (bind _returnvalue (`KismetMathLibrary.RandomFloatInRange` 0.8 1.1))
  (bind _returnvalue_2 (`KismetMathLibrary.RandomFloatInRange` 0.95 1.05))
  (bind _player (`self.Player`))
  (bind _player_2 (`self.Player`))
  (bind _returnvalue_roll (`KismetMathLibrary.BreakRotator` (`SceneComponent.K2_GetComponentRotation` (`/Game/Blueprints/BP_PlayerCharacter.Camera` _player_2))))
  (`|ExecutionSequence`
    (:`then_0`
      (if (`PlayerCharacter.bCanGrapple` _player)
        (set `self.StartedGrappling` true)
        (`/Engine/EditorBlueprintResources/StandardMacros.DoOnce` false :!label _label_2
          (:`Completed`
            (`GameplayStatics.PlaySoundAtLocation` "/Game/Audio/Sounds/Ambiance/PH_Drone.PH_Drone" (`self.K2_GetActorLocation` _player) (struct) _returnvalue_2 _returnvalue_2 0.0 null null null null)))
        (else
          (set `self.StartedGrappling` false)
          (goto _label_2 :!via `Reset`))))
    (:`then_1`
      (if (`/Game/Blueprints/BP_PlayerCharacter.Landed` (`self.Player`))
        (goto _label :!via `Reset`)))
    (:`then_2`
      ;[1 1 1] Play WallRun Sound
      (if (or (>= _returnvalue_roll 8.0) (<= _returnvalue_roll -8.0))
        (`/Engine/EditorBlueprintResources/StandardMacros.DoOnce` false :!label _label_3
          (:`Completed`
            (`GameplayStatics.PlaySoundAtLocation` "/Game/Audio/Sounds/Movement/PH_Springy_metal_landing.PH_Springy_metal_landing" (0.0 0.0 0.0) (struct) _returnvalue _returnvalue 0.0 null null _player_2 null)))
        (else
          (goto _label_3 :!via `Reset`))))))

(event `InputAction|Slide` :consume false
  (params (Key :type "Key Structure"))
  (bind _returnvalue (`KismetMathLibrary.RandomFloatInRange` 0.95 1.05))
  (:`Pressed`
    (`GameplayStatics.PlaySoundAtLocation` "/Game/Audio/Sounds/Movement/PH_SlideMaybe2Darker.PH_SlideMaybe2Darker" (`self.K2_GetActorLocation` (`self.Player`)) (struct) _returnvalue _returnvalue 0.0 null null null null)))

(event `Key|LeftMouseButton` :consume false
  (params (Key :type "Key Structure"))
  (bind _returnvalue (`KismetMathLibrary.RandomFloatInRange` 0.95 1.05))
  (:`Pressed`
    (`GameplayStatics.PlaySoundAtLocation` "/Game/FPWeapon/Audio/FirstPersonTemplateWeaponFire02.FirstPersonTemplateWeaponFire02" (`self.K2_GetActorLocation` (`self.Player`)) (struct) _returnvalue _returnvalue 0.0 null null null null)))

(event `InputAction|Deflect` :consume false
  (params (Key :type "Key Structure")))

(event `InputAction|Dash` :consume false
  (params (Key :type "Key Structure"))
  (bind _returnvalue (`KismetMathLibrary.RandomFloatInRange` 0.95 1.05))
  (bind _player (`self.Player`))
  (:`Pressed`
    (if (`PlayerCharacter.CanDash` _player)
      (`GameplayStatics.PlaySoundAtLocation` "/Game/Audio/Sounds/MSS_Dash_Sounds.MSS_Dash_Sounds" (`self.K2_GetActorLocation` _player) (struct) _returnvalue _returnvalue 0.0 null null null null))))

(fn `UserConstructionScript`)