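; Turret audio component that plays lock-on, turning and rocket launch sounds at its owner's location.
; On Tick, gaining player line of sight fires a one-shot lock-on cue with debug prints; while visible, large yaw changes trigger paired, pitch-randomized turning sounds, throttled by a delayed DoOnce reset.
; Launch audio runs on its own Delay timer, playing layered sounds when a BP_EnemyRocketTurret owner has the player in range and sight.
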(event `self.ReceiveTick`
  (params (DeltaSeconds :type "Float (single-precision)"))
  (bind _returnvalue (`self.GetOwner`))
  (bind _returnvalue_2 (`KismetMathLibrary.RandomFloatInRange` 0.9 1.05))
  (bind _returnvalue_3 (`self.GetOwner`))
  (bind _returnvalue_4 (`self.GetOwner`))
  (bind _outitem (`KismetArrayLibrary.Array_Random` (`self.Sounds`)))
  (bind _returnvalue_5 (`Actor.K2_GetActorLocation` (`self.GetOwner`)))
  (bind _yaw (`KismetMathLibrary.GetYawPitchFromVector` (`KismetMathLibrary.Conv_RotatorToVector` (`Actor.K2_GetActorRotation` _returnvalue_3))))
  (bind _returnvalue_6 (< (`KismetMathLibrary.Vector_Distance` (- (`Actor.K2_GetActorLocation` (`GameplayStatics.GetPlayerPawn` 0)) (`Actor.K2_GetActorLocation` (`self.GetOwner`)))) 2000.0))
  (bind _returnvalue_7 (- _yaw (`self.PreviousYaw`)))
  (`|ExecutionSequence`
    (:`then_0`
      (if (`Controller.LineOfSightTo` (`GameplayStatics.GetPlayerController` 0) _returnvalue_3 (0.0 0.0 0.0) false)
        (`|ExecutionSequence`
          (:`then_0`
            (`/Engine/EditorBlueprintResources/StandardMacros.DoOnce` false :!label _label
              (:`Completed`
                (set `self.PreviousYaw` _yaw)
                (`KismetSystemLibrary.PrintString` "Hello")
                (`KismetSystemLibrary.PrintString` (`KismetSystemLibrary.GetDisplayName` _returnvalue))
                (`GameplayStatics.PlaySoundAtLocation` "/Game/Audio/Sounds/Enemy_Obstacles/PH_LockOn.PH_LockOn" (`Actor.K2_GetActorLocation` _returnvalue) (struct) 1.0 1.0 0.0 "/Game/Audio/TurretAttenuation.TurretAttenuation" null null null))))
          (:`then_1`
            (if (or (<= _returnvalue_7 -15.0) (>= _returnvalue_7 15.0))
              (set `self.PreviousYaw` _yaw)
              (`/Engine/EditorBlueprintResources/StandardMacros.DoOnce` false :!label _label_2
                (:`Completed`
                  (`GameplayStatics.PlaySoundAtLocation` _outitem _returnvalue_5 (struct) 0.08 _returnvalue_2 0.0 "/Game/Audio/TurretAttenuation.TurretAttenuation" null null null)
                  (`KismetSystemLibrary.Delay` 0.1)
                  (`GameplayStatics.PlaySoundAtLocation` _outitem _returnvalue_5 (struct) 0.08 _returnvalue_2 0.0 "/Game/Audio/TurretAttenuation.TurretAttenuation" null null null)
                  (`KismetSystemLibrary.Delay` 1.2)
                  (goto _label_2 :!via `Reset`))))))
        (else
          (goto _label :!via `Reset`))))
    (:`then_1`
      (if _returnvalue_6
        (`KismetSystemLibrary.Delay` 2.0)
        (if (and (`Controller.LineOfSightTo` (`GameplayStatics.GetPlayerController` 0) _returnvalue_3 (0.0 0.0 0.0) false) _returnvalue_6 (== (`GameplayStatics.GetObjectClass` _returnvalue_4) "/Game/Blueprints/BP_EnemyRocketTurret.BP_EnemyRocketTurret_C"))
          (`GameplayStatics.PlaySoundAtLocation` "/Game/Audio/Sounds/MSS_RocketLaunch_Sounds.MSS_RocketLaunch_Sounds" (`Actor.K2_GetActorLocation` _returnvalue_4) (struct) 1.0 1.0 0.0 "/Game/Audio/TurretAttenuation.TurretAttenuation" null null null)
          (`KismetSystemLibrary.Delay` 0.1)
          (`GameplayStatics.PlaySoundAtLocation` "/Game/Audio/Sounds/MSS_RocketLaunch_Sounds.MSS_RocketLaunch_Sounds" (`Actor.K2_GetActorLocation` (`self.GetOwner`)) (struct) 1.0 0.7 0.0 "/Game/Audio/TurretAttenuation.TurretAttenuation" null null null))))))