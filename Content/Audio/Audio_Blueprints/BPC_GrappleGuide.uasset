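; Grapple guide audio Blueprint that plays a one-time sound cue once the player can perceive it.
; Each Tick checks whether the player controller has line of sight to it or the player character is within set horizontal and vertical distances.
; The first success passes a DoOnce, which is never reset, and sends the "Play" trigger to MSSCablebox.
; Tick also prints vertical player distance when the display name is BP_WeakSpot.
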(event `self.ReceiveTick`
  (params (DeltaSeconds :type "Float (single-precision)"))
  (bind _returnvalue (`GameplayStatics.GetPlayerCharacter` 0))
  (bind _returnvalue_2 (`Actor.GetVerticalDistanceTo` _returnvalue))
  (`|ExecutionSequence`
    (:`then_0`
      (if (== (`KismetSystemLibrary.GetDisplayName` self) "BP_WeakSpot")
        (`KismetSystemLibrary.PrintString` (`KismetStringLibrary.Conv_DoubleToString` _returnvalue_2))))
    (:`then_1`
      (if (or (`Controller.LineOfSightTo` (`GameplayStatics.GetPlayerController` 0) self (0.0 0.0 0.0) false) (and (< (`Actor.GetHorizontalDistanceTo` _returnvalue) 500.0) (< _returnvalue_2 300.0)))
        (`/Engine/EditorBlueprintResources/StandardMacros.DoOnce` false
          (:`Completed`
            (`AudioParameterControllerInterface.SetTriggerParameter` (`self.MSS_Cablebox`) "Play")))))))