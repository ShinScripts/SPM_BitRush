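; Rocket launch audio logic that fires Beep and LaunchRocket triggers on its owner's AudioComponent when the player is nearby with line of sight.
; Tick checks sight and distance, with a DoOnce playing the first delayed beep-then-launch sequence.
; A parallel Delay throttles the repeating cycle, rechecking both conditions before triggering launch, then beep.
; Older PlaySoundAtLocation calls using the rocket MetaSound remain unconnected.
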(event `self.ReceiveTick`
  (params (DeltaSeconds :type "Float (single-precision)"))
  (bind _returnvalue (`Actor.GetComponentByClass` (`self.GetOwner`) "/Script/Engine.AudioComponent"))
  (bind _returnvalue_2 (and (`Controller.LineOfSightTo` (`GameplayStatics.GetPlayerController` 0) (`self.GetOwner`) (0.0 0.0 0.0) false) (< (`KismetMathLibrary.Vector_Distance` (- (`Actor.K2_GetActorLocation` (`GameplayStatics.GetPlayerPawn` 0)) (`Actor.K2_GetActorLocation` (`self.GetOwner`)))) 2000.0)))
  (if _returnvalue_2
    (`|ExecutionSequence`
      (:`then_0`
        (`/Engine/EditorBlueprintResources/StandardMacros.DoOnce` false
          (:`Completed`
            (`KismetSystemLibrary.Delay` 1.0)
            (`KismetSystemLibrary.PrintString` "beepFirst")
            (`AudioParameterControllerInterface.SetTriggerParameter` _returnvalue "Beep")
            (`KismetSystemLibrary.Delay` 1.0)
            (`AudioParameterControllerInterface.SetTriggerParameter` _returnvalue "LaunchRocket"))))
      (:`then_1`
        (`KismetSystemLibrary.Delay` 2.0)
        (if _returnvalue_2
          (`AudioParameterControllerInterface.SetTriggerParameter` _returnvalue "LaunchRocket")
          (`KismetSystemLibrary.Delay` 1.0)
          (`AudioParameterControllerInterface.SetTriggerParameter` _returnvalue "Beep"))))))