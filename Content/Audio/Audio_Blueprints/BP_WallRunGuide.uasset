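; Component on SoundViewpoint actors that plays an electric guide sound, apparently to point players toward wall runs.
; Each Tick, if the player has line of sight and is in range and CanPlay is set, it plays a layered cue (normal, then delayed low-pitched fade-in) at the owner, with a cooldown and play-count limit.
; Playing sets DidPlay, which owners also copy from nearby viewpoints.
; Unwired branches hold unused overlap-suppression and debug logic.
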(event `self.ReceiveTick`
  (params (DeltaSeconds :type "Float (single-precision)"))
  (bind _returnvalue (`Actor.K2_GetActorLocation` (`self.Closest`)))
  (`|ExecutionSequence`
    (:`then_0`
      (if (and (`Controller.LineOfSightTo` (`GameplayStatics.GetPlayerController` 0) (`self.GetOwner`) (0.0 0.0 0.0) false) (<= (`self.PlayCount`) 2) (< (`KismetMathLibrary.Vector_Distance` (- (`Actor.K2_GetActorLocation` (`GameplayStatics.GetPlayerPawn` 0)) (`Actor.K2_GetActorLocation` (`self.GetOwner`)))) 3000.0))
        (bind _assound_viewpoint (cast `/Game/Audio/Audio_Blueprints/SoundViewpoint` (`self.GetOwner`)))
        (if (`/Game/Audio/Audio_Blueprints/SoundViewpoint.CanPlay` _assound_viewpoint)
          (`/Engine/EditorBlueprintResources/StandardMacros.DoOnce` false :!label _label
            (:`Completed`
              (`|ExecutionSequence`
                (:`then_0`
                  (`GameplayStatics.PlaySoundAtLocation` "/Game/Audio/Sounds/Other/PH_CoolElectric.PH_CoolElectric" _returnvalue (struct) 0.6 1.0 0.0 "/Game/Audio/GuideSoundAttenuation.GuideSoundAttenuation" null null null)
                  (`KismetSystemLibrary.Delay` 0.4)
                  (bind _returnvalue_2 (`GameplayStatics.SpawnSoundAtLocation` "/Game/Audio/Sounds/Other/PH_CoolElectric.PH_CoolElectric" _returnvalue (struct) 1.0 0.1 0.0 "/Game/Audio/GuideSoundAttenuation.GuideSoundAttenuation" null))
                  (`AudioComponent.FadeIn` _returnvalue_2 0.1 1.0 0.4 "Linear")
                  (set `self.PlayCount` (+ (`self.PlayCount`) 1)))
                (:`then_1`
                  (`/Engine/EditorBlueprintResources/StandardMacros.DoOnce` false
                    (:`Completed`
                      (bind _assound_viewpoint_2 (cast `/Game/Audio/Audio_Blueprints/SoundViewpoint` (`self.GetOwner`)))
                      (set `/Game/Audio/Audio_Blueprints/SoundViewpoint.DidPlay` true _assound_viewpoint_2))))
                (:`then_2`
                  (`KismetSystemLibrary.Delay` 1.0)
                  (`|ExecutionSequence`
                    (:`then_0`
                      (goto _label :!via `Reset`))
                    (:`then_1`
                      (if (== (`self.PlayCount`) 5)
                        _))))))))))
    (:`then_1`
      (for _array_element (`self.WallSounds`)
        (bind _returnvalue_3 (`Actor.GetDistanceTo` _array_element (`self.GetOwner`)))
        (if (and (< _returnvalue_3 620.0) (!= _returnvalue_3 0.0))
          (if (`/Game/Audio/Audio_Blueprints/SoundViewpoint.DidPlay` _array_element)
            (bind _assound_viewpoint_3 (cast `/Game/Audio/Audio_Blueprints/SoundViewpoint` (`self.GetOwner`)))
            (set `/Game/Audio/Audio_Blueprints/SoundViewpoint.DidPlay` true _assound_viewpoint_3)))))))

(event `self.ReceiveBeginPlay`
  (bind _assound_viewpoint (cast `/Game/Audio/Audio_Blueprints/SoundViewpoint` (`self.GetOwner`)))
  (set `self.Closest` _assound_viewpoint)
  (bind _outactors (`GameplayStatics.GetAllActorsOfClass` "/Game/Audio/Audio_Blueprints/SoundViewpoint.SoundViewpoint_C"))
  (set `self.WallSounds` _outactors))