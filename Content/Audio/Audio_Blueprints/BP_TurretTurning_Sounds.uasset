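; Component that plays a turret's lock-on and turning sounds by sending trigger parameters to the owner's AudioComponent.
; Each tick it checks the first player controller's line of sight to the owner, firing "LockOn" once whenever sight is gained.
; While sight holds, a large yaw change from the stored value updates it and fires "Turn", throttled by a delay-reset DoOnce.
; The yaw difference is not wrapped at ±180 degrees.
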(event `self.ReceiveTick`
  (params (DeltaSeconds :type "Float (single-precision)"))
  (bind _returnvalue (`self.GetOwner`))
  (bind _returnvalue_2 (`Actor.GetComponentByClass` _returnvalue "/Script/Engine.AudioComponent"))
  (bind _yaw (`KismetMathLibrary.GetYawPitchFromVector` (`KismetMathLibrary.Conv_RotatorToVector` (`Actor.K2_GetActorRotation` _returnvalue))))
  (bind _returnvalue_3 (- _yaw (`self.PreviousYaw`)))
  (if (`Controller.LineOfSightTo` (`GameplayStatics.GetPlayerController` 0) _returnvalue (0.0 0.0 0.0) false)
    (`|ExecutionSequence`
      (:`then_0`
        (`/Engine/EditorBlueprintResources/StandardMacros.DoOnce` false :!label _label
          (:`Completed`
            (set `self.PreviousYaw` _yaw)
            (`AudioParameterControllerInterface.SetTriggerParameter` _returnvalue_2 "LockOn"))))
      (:`then_1`
        (if (or (<= _returnvalue_3 -30.0) (>= _returnvalue_3 30.0))
          (set `self.PreviousYaw` _yaw)
          (`/Engine/EditorBlueprintResources/StandardMacros.DoOnce` false :!label _label_2
            (:`Completed`
              (`AudioParameterControllerInterface.SetTriggerParameter` _returnvalue_2 "Turn")
              (`KismetSystemLibrary.Delay` 1.2)
              (goto _label_2 :!via `Reset`))))))
    (else
      (goto _label :!via `Reset`))))