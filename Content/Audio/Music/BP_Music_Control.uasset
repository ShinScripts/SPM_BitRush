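; BP_Music_Control is a keyboard-driven controller for switching music tracks and adjusting volume on a MetaSound music player.
; Any key whose display name is in ValidInputs becomes the SelectMusic index and fires the ChangeMusic trigger, with track 5 getting a different start time.
; Add and Subtract step a clamped Volume into the MetaSound's Volume parameter.
; Key presses and volume changes print debug text.
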(event `Key|AnyKey` :consume false
  (params (Key :type "Key Structure"))
  (bind _returnvalue (`KismetInputLibrary.Key_GetDisplayName` Key))
  (bind _mss_music_player (`self.MSS_Music_Player`))
  (bind _mss_music_player_2 (`self.MSS_Music_Player`))
  (bind _returnvalue_2 (`KismetTextLibrary.Conv_TextToString` _returnvalue))
  (bind _returnvalue_3 (`KismetArrayLibrary.Array_Contains` (`self.validInputs`) _returnvalue_2))
  (bind _returnvalue_4 (`KismetStringLibrary.Conv_StringToInt` _returnvalue_2))
  (:`Pressed`
    (`KismetSystemLibrary.PrintText` _returnvalue)
    (`KismetSystemLibrary.PrintString` _returnvalue_2)
    (`KismetSystemLibrary.PrintString` (`KismetStringLibrary.Conv_BoolToString` _returnvalue_3))
    (if _returnvalue_3
      (if (== _returnvalue_4 5)
        (`AudioComponent.SetFloatParameter` _mss_music_player_2 "SetStartTime" 1.0)
        (else
          (`AudioComponent.SetFloatParameter` _mss_music_player_2 "SetStartTime" 0.0)))
      (`AudioParameterControllerInterface.SetIntParameter` _mss_music_player "SelectMusic" _returnvalue_4)
      (`AudioParameterControllerInterface.SetTriggerParameter` _mss_music_player "ChangeMusic"))))

(event `Key|Subtract` :consume false
  (params (Key :type "Key Structure"))
  (bind _volume (`self.Volume`))
  (:`Pressed`
    (bind _output_get (set `self.Volume` (`KismetMathLibrary.FClamp` (- _volume 0.05))))
    (`AudioComponent.SetFloatParameter` (`self.MSS_Music_Player`) "Volume" _output_get)
    (`KismetSystemLibrary.PrintString` (`KismetStringLibrary.Conv_DoubleToString` _volume) :!label _label)))

(event `Key|Add` :consume false
  (params (Key :type "Key Structure"))
  (:`Pressed`
    (bind _output_get (set `self.Volume` (`KismetMathLibrary.FClamp` (+ (`self.Volume`) 0.05))))
    (`AudioComponent.SetFloatParameter` (`self.MSS_Music_Player`) "Volume" _output_get)
    (goto _label)))

(fn `UserConstructionScript`)