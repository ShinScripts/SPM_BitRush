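; Rocket projectile actor that homes in on the player pawn and destroys itself after about five seconds.
; Each tick moves it toward the player at constant speed with VInterpToConstant and smoothly turns it to face them with RInterpTo.
; The same tick chain runs a Delay into DestroyActor, serving as the lifetime timer.
; A hit on the Cube component only prints a debug string, with no damage or destruction.
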(event `self.Cube.OnComponentHit`
  (params (HitComponent :type "PrimitiveComponent Object Reference") (OtherActor :type "Actor Object Reference") (OtherComp :type "PrimitiveComponent Object Reference") (NormalImpulse :type "Vector Structure") (Hit :type "HitResult Structure (by ref)"))
  (`KismetSystemLibrary.PrintString` "Hello"))

(event `self.ReceiveTick`
  (params (DeltaSeconds :type "Float (single-precision)"))
  (bind _returnvalue (`self.K2_GetActorLocation`))
  (bind _returnvalue_2 (`self.K2_GetActorLocation` (`GameplayStatics.GetPlayerPawn` 0)))
  (if true
    (`self.K2_SetActorLocationAndRotation` (`KismetMathLibrary.VInterpTo_Constant` _returnvalue _returnvalue_2 DeltaSeconds 500.0) (`KismetMathLibrary.RInterpTo` (`self.K2_GetActorRotation`) (`KismetMathLibrary.Conv_VectorToRotator` (- _returnvalue_2 _returnvalue)) DeltaSeconds 10.0))
    (`KismetSystemLibrary.Delay` 5.0)
    (`self.K2_DestroyActor`)))

(fn `UserConstructionScript`)