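; Player character Blueprint for a first-person movement shooter with jumping, wall running, dashing, grappling and a hitscan gun that destroys tagged targets.
; Input and Tick watch movement components and camera roll to fire MetaSound triggers and one-shot sounds through DoOnce gates, and drive Chameleon speed lines from velocity.
; Tick also selects the nearest SoundViewpoint wall-run cue.
; Debug keys handle mute, music track and volume, restart, and teleporting to cheat locations.
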(event `InputAction|Jump` :consume false :overrideparent false
  (params (Key :type "Key Structure"))
  ;[1 1 1 1 308] Sound
  ;;[1 1 1] JumpSounds
  (:`Pressed`
    (if (not (`self.Mute`))
      (`/Engine/EditorBlueprintResources/StandardMacros.DoOnce` false :!label _label
        (:`Completed`
          (`AudioParameterControllerInterface.SetTriggerParameter` (`self.MSS_Jump_Sounds`) "Jump")
          (bind _output_get (set `self.DidJump` true)))))))

(event `self.ReceiveTick`
  (params (DeltaSeconds :type "Float (single-precision)"))
  (bind _returnvalue (`KismetMathLibrary.RandomFloatInRange` 0.8 1.1))
  (bind _returnvalue_2 (`self.K2_GetActorLocation`))
  (bind _returnvalue_3 (`KismetMathLibrary.RandomFloatInRange` 0.95 1.05))
  (bind _charactermovement (`self.CharacterMovement`))
  (bind _wallsounds (`self.WallSounds`))
  (bind _mss_playergun_sounds (`self.MSS_PlayerGun_Sounds`))
  (bind _chameleon (`self.Chameleon`))
  (bind (_grapplecomponent_bcangrapple _grapplecomponent_bisgrappling) (break `GrappleComponent` (`self.GrappleComponent`)))
  (bind _wallsounds_2 (`self.WallSounds`))
  (bind (_dashcomponent_dashcooldown _dashcomponent_dashcurrentcooldown _dashcomponent_bisdashing) (break `DashComponent` (`self.DashComponent`)))
  (bind _closestwall (`self.ClosestWall`))
  (bind _wallsounds_3 (`self.WallSounds`))
  (bind _returnvalue_4 (`NavMovementComponent.IsFalling` (`self.CharacterMovement`)))
  (bind _returnvalue_roll (`KismetMathLibrary.BreakRotator` (`SceneComponent.K2_GetComponentRotation` (`self.Camera`))))
  (bind _returnvalue_5 (`KismetMathLibrary.VSize` (`MovementComponent.Velocity` _charactermovement)))
  (bind _returnvalue_6 (not _returnvalue_4))
  (bind _returnvalue_7 (* _returnvalue_5 0.0002))
  (`|ExecutionSequence`
    (:`then_0`
      (`/Game/Chameleon/Chameleon.InitChameleon` _chameleon)
      (`/Game/Chameleon/Chameleon.Speed Lines Func` _chameleon (or (> _returnvalue_5 (+ (`MovementComponent.GetMaxSpeed` _charactermovement) 300.0)) _dashcomponent_bisdashing))
      (set `/Game/Chameleon/Chameleon.Speed Lines Line Width` 0.3 _chameleon)
      (set `/Game/Chameleon/Chameleon.Speed Lines Intensity` _returnvalue_7 _chameleon)
      (set `/Game/Chameleon/Chameleon.Speed Lines Mask Radius` (- (+ _returnvalue_7 3.0) _returnvalue_7) _chameleon))
    (:`then_1`
      ;[1 1 1 1 308] Sound
      (`|ExecutionSequence`
        (:`then_0`
          (if (not (`self.Mute`))
            ;;[1 1 1] GrappleSounds
            (`|ExecutionSequence`
              (:`then_0`
                (if _grapplecomponent_bcangrapple
                  (if (not _grapplecomponent_bisgrappling)
                    (`/Engine/EditorBlueprintResources/StandardMacros.DoOnce` false :!label _label_2
                      (:`Completed`
                        (`GameplayStatics.PlaySoundAtLocation` "/Game/Audio/Sounds/Ambiance/PH_Drone.PH_Drone" _returnvalue_2 (struct) _returnvalue_3 _returnvalue_3 0.0 null null null null))))
                  (else
                    (`KismetSystemLibrary.Delay` 5.0)
                    (goto _label_2 :!via `Reset`))))
              (:`then_1`
                (if _grapplecomponent_bisgrappling
                  (`/Engine/EditorBlueprintResources/StandardMacros.DoOnce` false :!label _label_3
                    (:`Completed`
                      (`GameplayStatics.PlaySoundAtLocation` "/Game/Audio/Sounds/Movement/PH_RoboStep.PH_RoboStep" _returnvalue_2 (struct) _returnvalue_3 _returnvalue_3 0.0 null null null null)))
                  (else
                    (goto _label_3 :!via `Reset`)))))))
        (:`then_1`
          ;;[1 1 1] JumpSounds
          (if (not _returnvalue_4)
            (goto _label :!via `Reset`)))
        (:`then_2`
          (if (and (stale `InputAction|Jump` _output_get) _returnvalue_6)
            (if (not (`self.Mute`))
              (`AudioParameterControllerInterface.SetTriggerParameter` (`self.MSS_Jump_Sounds`) "Land")
              (set `self.DidJump` false))))
        (:`then_3`
          (if _returnvalue_6
            (goto _label_4 :!via `Reset`)))
        (:`then_4`
          (if (and _returnvalue_4 (not (`self.DidJump`)))
            (`/Engine/EditorBlueprintResources/StandardMacros.DoOnce` false :!label _label_4
              (:`Completed`
                (if (not (`self.Mute`))
                  (`AudioParameterControllerInterface.SetTriggerParameter` (`self.MSS_Jump_Sounds`) "Land"))))))
        (:`then_5`
          ;;[1 1 1] Play WallRun Sound
          (if (or (>= _returnvalue_roll 8.0) (<= _returnvalue_roll -8.0))
            (`/Engine/EditorBlueprintResources/StandardMacros.DoOnce` false :!label _label_5
              (:`Completed`
                (set `self.DoneWallRunning` false)
                (set `self.StartedWallRun` true)
                (if (not (`self.Mute`))
                  (`GameplayStatics.PlaySoundAtLocation` "/Game/Audio/Sounds/Movement/PH_Springy_metal_landing.PH_Springy_metal_landing" (`self.K2_GetActorLocation`) (struct) _returnvalue _returnvalue 0.0 null null null null))))
            (else
              (set `self.DoneWallRunning` false)
              (if (`self.StartedWallRun`)
                (set `self.DoneWallRunning` true)
                (set `self.StartedWallRun` false)
                (goto _label_5 :!via `Reset`)))))
        (:`then_6`
          ;;[1 1 1] GunSounds
          (if (`self.isRealoading`)
            (`AudioComponent.SetFloatParameter` _mss_playergun_sounds "ClickVolume" 0.0)
            (else
              (`AudioComponent.SetFloatParameter` _mss_playergun_sounds "ClickVolume" 1.0)))
          (if (not (and (`self.isRealoading`) (== (`self.CurrentMagAmmo`) 0)))
            (set `self.isRealoading` false)))
        (:`then_7`
          ;;[1 1 1] MusicControll
          (if (`self.Mute`)
            (`AudioComponent.SetFloatParameter` (`self.MSS_Music_Player`) "Volume" 0.0)))
        (:`then_8`
          ;;[1 1 1] WallRunGuide
          (`/Engine/EditorBlueprintResources/StandardMacros.DoOnce` false :!label _label_6
            (:`Completed`
              (for _array_element _wallsounds_2
                (`|ExecutionSequence`
                  (:`then_0`
                    (`/Engine/EditorBlueprintResources/StandardMacros.DoOnce` false :!label _label_7
                      (:`Completed`
                        (set `self.ClosestWall` (`KismetArrayLibrary.Array_Random` _wallsounds_2)))))
                  (:`then_1`
                    (set `self.Current` _array_element)
                    (if (> (`self.GetDistanceTo` (`self.ClosestWall`)) (`self.GetDistanceTo` (`self.Current`)))
                      (set `self.ClosestWall` (`self.Current`))))))
              (if (not (`/Game/Audio/Audio_Blueprints/SoundViewpoint.DidPlay` _closestwall))
                (set `/Game/Audio/Audio_Blueprints/SoundViewpoint.CanPlay` true _closestwall)))))
        (:`then_9`
          (if (`self.DoneWallRunning`)
            (`KismetSystemLibrary.PrintString` "Reset")
            (`|ExecutionSequence`
              (:`then_0`
                (`KismetSystemLibrary.Delay` 2.0)
                (if (`self.StartedWallRun`)
                  (for _array_element_2 _wallsounds_3
                    (`|ExecutionSequence`
                      (:`then_0`
                        (set `self.ClosestWall` (`KismetArrayLibrary.Array_Random` _wallsounds_3)))
                      (:`then_1`
                        (set `self.Current` _array_element_2)
                        (if (> (`self.GetDistanceTo` (`self.ClosestWall`)) (`self.GetDistanceTo` (`self.Current`)))
                          (set `self.ClosestWall` (`self.Current`))))))
                  (set `/Game/Audio/Audio_Blueprints/SoundViewpoint.DidPlay` true (`self.ClosestWall`))
                  (else
                    (goto _label_6 :!via `Reset`))))
              (:`then_1`
                (goto _label_7 :!via `Reset`)))))
        (:`then_10`
          (for _array_element_3 _wallsounds
            (if (`/Game/Audio/Audio_Blueprints/SoundViewpoint.DidPlay` _array_element_3)
              (`KismetSystemLibrary.PrintString` "removing")
              (`KismetSystemLibrary.PrintString` (`KismetSystemLibrary.GetDisplayName` _array_element_3))
              (`KismetArrayLibrary.Array_RemoveItem` _wallsounds _array_element_3))))))))

(event `Key|End`
  (params (Key :type "Key Structure"))
  ;[1 1 1] Restart Level
  (:`Pressed`
    (`self.K2_SetActorLocation` (`self.StartLocation`))))

(event `InputAction|Shoot`
  (params (Key :type "Key Structure"))
  (:`Pressed`
    (if (> (`self.CurrentMagAmmo`) 0)
      (set `self.CurrentMagAmmo` (- (`self.CurrentMagAmmo`) 1))
      (`self.FireProjectile`)
      (bind _returnvalue (`NiagaraFunctionLibrary.SpawnSystemAttached` "/Game/Particles/MuzzleFlash.MuzzleFlash" (`self.GunWithMuzzleJoint`) "Muzzle" (0.0 0.0 0.0) (struct :`Roll` 90.0) "KeepRelativeOffset"))
      (`SceneComponent.SetWorldScale3D` _returnvalue (0.03 0.03 0.03)))))

(event `Key|Section` :consume false :overrideparent false
  (params (Key :type "Key Structure"))
  (bind _mss_music_player (`self.MSS_Music_Player`))
  ;[1 1 1 1 308] Sound
  ;;[1 1 1] MutePlayerSounds
  (:`Pressed`
    (`/Engine/EditorBlueprintResources/StandardMacros.FlipFlop`
      (:`A`
        (set `self.Mute` true)
        (`AudioComponent.SetFloatParameter` _mss_music_player "Volume" 0.0))
      (:`B`
        (set `self.Mute` false)
        (`AudioComponent.SetFloatParameter` _mss_music_player "Volume" (`self.Volume`))))))

(event `Key|LeftMouseButton` :consume false :overrideparent false
  (params (Key :type "Key Structure"))
  (bind _mss_playergun_sounds (`self.MSS_PlayerGun_Sounds`))
  ;[1 1 1 1 308] Sound
  ;;[1 1 1] GunSounds
  (:`Pressed`
    (if (`self.Mute`)
      _
      (elif (> (`self.CurrentMagAmmo`) 0)
        (`AudioParameterControllerInterface.SetTriggerParameter` _mss_playergun_sounds "Fire")
        (`|ExecutionSequence`
          (:`then_0`
            (`/Engine/EditorBlueprintResources/StandardMacros.DoOnce` false :!label _label_8
              (:`Completed`
                (set `self.RandomNumber` (`KismetMathLibrary.RandomIntegerInRange` 3 8)))))
          (:`then_1`
            (bind _output_get (set `self.ShotCount` (+ (`self.ShotCount`) 1)))
            (if (== _output_get (`self.RandomNumber`))
              (`|ExecutionSequence`
                (:`then_0`
                  (goto _label_8 :!via `Reset`))
                (:`then_1`
                  (set `self.ShotCount` 0)
                  (`AudioParameterControllerInterface.SetTriggerParameter` (`self.MSS_PlayerGun_Sounds`) "DropShell"))))))
        (else
          (`AudioParameterControllerInterface.SetTriggerParameter` _mss_playergun_sounds "Click"))))))

(event `self.ReceiveBeginPlay`
  (`|ExecutionSequence`
    (:`then_0`
      (set `self.StartLocation` (`self.K2_GetActorLocation`))
      (bind _outactors (`GameplayStatics.GetAllActorsWithTag` "ActorDestroy"))
      (set `self.actors` _outactors)
      (bind _returnvalue (`GameplayStatics.GetActorOfClass` "/Game/Chameleon/Chameleon.Chameleon_C"))
      (set `self.Chameleon` _returnvalue))
    (:`then_1`
      ;[1 1 1 1 308] Sound
      (bind _outactors_2 (`GameplayStatics.GetAllActorsOfClass` "/Game/Audio/Audio_Blueprints/SoundViewpoint.SoundViewpoint_C"))
      (set `self.WallSounds` _outactors_2))))

(event `InputAction|Dash` :consume false :overrideparent false
  (params (Key :type "Key Structure"))
  (bind (_dashcomponent_dashcooldown _dashcomponent_dashcurrentcooldown _dashcomponent_bisdashing) (break `DashComponent` (`self.DashComponent`)))
  ;[1 1 1 1 308] Sound
  ;;[1 1 1] DashSounds
  (:`Pressed`
    (if (`self.Mute`)
      _
      (elif _dashcomponent_bisdashing
        (`/Engine/EditorBlueprintResources/StandardMacros.DoOnce` false :!label _label_9
          (:`Completed`
            (`KismetSystemLibrary.PrintString` "dash")
            (`AudioParameterControllerInterface.SetTriggerParameter` (`self.MSS_Dash_Sounds`) "Dash")))
        (else
          (goto _label_9 :!via `Reset`))))))

(event `InputAction|Jump`
  (params (Key :type "Key Structure"))
  (bind _wallrunmovement (`self.WallRunMovement`))
  (bind _wallrunmovement_2 (`self.WallRunMovement`))
  ;[1 1 1] Event: Jump
  (:`Pressed`
    (if (or (`WallRunMovementComponent.OnRightSide` _wallrunmovement_2) (`WallRunMovementComponent.OnLeftSide` _wallrunmovement_2))
      (`WallRunMovementComponent.JumpOffWall` _wallrunmovement self)
      (`KismetSystemLibrary.Delay` 0.2)
      (set `WallRunMovementComponent.IsJumpingOffWall` false _wallrunmovement)
      (else
        (`self.Jump`)))))

(event `Key|R` :consume false :overrideparent false
  (params (Key :type "Key Structure"))
  ;[1 1 1 1 308] Sound
  ;;[1 1 1] EeloadSounds
  (:`Pressed`
    (if (`self.Mute`)
      _
      (elif (or (== (`self.CurrentMagAmmo`) 0) (!= 0 8))
        (`AudioParameterControllerInterface.SetTriggerParameter` (`self.MSS_PlayerGun_Sounds`) "Reloading")
        (set `self.isRealoading` true)))))

(event `Key|AnyKey`
  (params (Key :type "Key Structure"))
  (bind _returnvalue (`KismetTextLibrary.Conv_TextToString` (`KismetInputLibrary.Key_GetDisplayName` Key)))
  (bind _returnvalue_2 (`KismetStringLibrary.Conv_StringToInt` _returnvalue))
  ;[1 1 1] Cheat Location
  (:`Pressed`
    (if (`KismetStringLibrary.IsNumeric` _returnvalue)
      (bind _returnvalue_3 (`GameplayStatics.GetActorOfClass` "/Script/Bit_Rush.CheatLocationManager"))
      (bind _locations (`CheatLocationManager.Locations` _returnvalue_3))
      (if (< _returnvalue_2 (`KismetArrayLibrary.Array_Length` _locations))
        (`self.K2_SetActorLocation` (`|GetArrayItem` _locations _returnvalue_2))))))

(event `InputAction|Slide` :consume false :overrideparent false
  (params (Key :type "Key Structure"))
  (bind _returnvalue (`KismetMathLibrary.RandomFloatInRange` 0.95 1.05))
  ;[1 1 1 1 308] Sound
  ;;[1 1 1] SlideSound
  (:`Pressed`
    (if (not (`self.Mute`))
      (`GameplayStatics.PlaySoundAtLocation` "/Game/Audio/Sounds/MSS_Slide_Sounds.MSS_Slide_Sounds" (`self.K2_GetActorLocation`) (struct) _returnvalue _returnvalue 0.0 null null null null))))

(event `InputAction|Deflect` :consume false :overrideparent false
  (params (Key :type "Key Structure"))
  ;[1 1 1 1 308] Sound
  ;;[1 1 1] DeflectSound
  (:`Pressed`
    (if (not (`self.Mute`))
      (`GameplayStatics.PlaySoundAtLocation` "/Game/Audio/Sounds/MSS_Deflect_Sounds.MSS_Deflect_Sounds" (`self.K2_GetActorLocation`) (struct) 1.0 (`KismetMathLibrary.RandomFloatInRange` 0.95 1.05) 0.0 null null null null))))

(event `Key|AnyKey` :consume false :overrideparent false
  (params (Key :type "Key Structure"))
  (bind _mss_music_player (`self.MSS_Music_Player`))
  (bind _mss_music_player_2 (`self.MSS_Music_Player`))
  (bind _returnvalue (`KismetStringLibrary.Conv_StringToInt` (`KismetTextLibrary.Conv_TextToString` (`KismetInputLibrary.Key_GetDisplayName` Key))))
  ;[1 1 1 1 308] Sound
  ;;[1 1 1] MusicControll
  (:`Pressed`
    (if (`KismetArrayLibrary.Array_Contains` (`self.ValidInputs`) Key)
      (if (== _returnvalue 5)
        (`AudioComponent.SetFloatParameter` _mss_music_player_2 "SetStartTime" 1.0)
        (else
          (`AudioComponent.SetFloatParameter` _mss_music_player_2 "SetStartTime" 0.0)))
      (`AudioParameterControllerInterface.SetIntParameter` _mss_music_player "SelectMusic" _returnvalue)
      (`AudioParameterControllerInterface.SetTriggerParameter` _mss_music_player "ChangeMusic"))))

(event `Key|Subtract` :consume false
  (params (Key :type "Key Structure"))
  ;[1 1 1 1 308] Sound
  ;;[1 1 1] MusicControll
  (:`Pressed`
    (bind _output_get (set `self.Volume` (`KismetMathLibrary.FClamp` (- (`self.Volume`) 0.05))))
    (`AudioComponent.SetFloatParameter` (`self.MSS_Music_Player`) "Volume" _output_get)))

(event `Key|Add` :consume false
  (params (Key :type "Key Structure"))
  ;[1 1 1 1 308] Sound
  ;;[1 1 1] MusicControll
  (:`Pressed`
    (bind _output_get (set `self.Volume` (`KismetMathLibrary.FClamp` (+ (`self.Volume`) 0.05))))
    (`AudioComponent.SetFloatParameter` (`self.MSS_Music_Player`) "Volume" _output_get)))

(fn `FireProjectile`
  (bind _camera (`self.Camera`))
  (bind _returnvalue (`SceneComponent.K2_GetComponentLocation` _camera))
  (bind (_outhit _returnvalue_2) (`KismetSystemLibrary.LineTraceSingle` :`Start` _returnvalue :`End` (+ _returnvalue (* (`SceneComponent.GetForwardVector` _camera) (`self.GunRange`))) :`TraceChannel` "TraceTypeQuery1" :`DrawDebugType` "ForDuration" :`DrawTime` 1.0))
  (bind (_bblockinghit _binitialoverlap _time _distance _location _impactpoint _normal) (`GameplayStatics.BreakHitResult` _outhit))
  (`NiagaraFunctionLibrary.SpawnSystemAtLocation` "/Game/Particles/WallHit.WallHit" _impactpoint (`KismetMathLibrary.Conv_VectorToRotator` _normal) (0.1 0.1 0.1))
  (if _returnvalue_2
    (bind (_outhit_2 _returnvalue_3) (`KismetSystemLibrary.SphereTraceSingle` :`Start` _impactpoint :`End` _impactpoint :`Radius` (`self.GunRadius`) :`TraceChannel` "TraceTypeQuery1" :`DrawDebugType` "ForDuration" :`DrawTime` 1.0))
    (if _returnvalue_3
      (if (`KismetArrayLibrary.Array_Contains` (`Actor.Tags` (`.HitActor` (`GameplayStatics.BreakHitResult` _outhit_2))) "WeakSpot")
        (bind _asbp_weak_spot (cast `/Game/Blueprints/BP_WeakSpot` (`.HitActor` (`GameplayStatics.BreakHitResult` _outhit_2))))
        (`/Game/Blueprints/BP_WeakSpot.DestroyTurrets` _asbp_weak_spot)
        (else
          (bind _componenttags (`ActorComponent.ComponentTags` (`.HitComponent` (`GameplayStatics.BreakHitResult` _outhit_2))))
          (if (`KismetArrayLibrary.Array_Contains` _componenttags "DestroyLaser")
            (for _array_element (`self.actors`)
              (`self.K2_DestroyActor` _array_element))
            (elif (`KismetArrayLibrary.Array_Contains` _componenttags "Destroyable")
              (`self.K2_DestroyActor` (`.HitActor` (`GameplayStatics.BreakHitResult` _outhit_2))))))))))

(fn `NewFunction`)

(fn `UserConstructionScript`)