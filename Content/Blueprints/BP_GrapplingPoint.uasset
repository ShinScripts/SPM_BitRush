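; BP_GrapplingPoint is a world grapple anchor that shows an icon when the player can grapple to it.
; It caches the BP_PlayerCharacter on BeginPlay.
; Each tick, the GrapplingIcon turns at a constant rate to face the player, and its visibility mirrors the PlayerCanGrapple flag of GrapplingFeedback.
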(event `self.ReceiveBeginPlay`
  (bind _asbp_player_character (cast `/Game/Blueprints/BP_PlayerCharacter` (`GameplayStatics.GetPlayerCharacter` 0)))
  (set `self.PlayerReference` _asbp_player_character))

(event `self.ReceiveTick`
  (params (DeltaSeconds :type "Float (single-precision)"))
  (bind _grapplingicon (`self.GrapplingIcon`))
  (bind (_returnvalue_roll _returnvalue_pitch _returnvalue_yaw) (`KismetMathLibrary.BreakRotator` (`KismetMathLibrary.RInterpTo_Constant` (`SceneComponent.K2_GetComponentRotation` _grapplingicon) (`KismetMathLibrary.FindLookAtRotation` (`SceneComponent.K2_GetComponentLocation` _grapplingicon) (`self.K2_GetActorLocation` (`self.PlayerReference`))) DeltaSeconds 200.0)))
  (`SceneComponent.K2_SetWorldRotation` _grapplingicon (`KismetMathLibrary.MakeRotator` _returnvalue_roll _returnvalue_pitch _returnvalue_yaw) false false)
  (`SceneComponent.SetVisibility` _grapplingicon (`GrapplingFeedbackComponent.PlayerCanGrapple` (`self.GrapplingFeedback`)) false))

(fn `UserConstructionScript`)