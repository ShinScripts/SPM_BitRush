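; Homing rocket projectile that chases the player, turns to face them and self-destructs after a short delay.
; Overlap ignores rocket turrets and the player, while anything else triggers an explosion and destroys the rocket.
; Player hits are resolved on Tick, using the overlap event's OtherActor and a capsule overlap check to deal damage, spawn a smaller explosion and destroy it.
; A deflector box check exists but never runs.
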(event `self.ReceiveActorBeginOverlap`
  (params (OtherActor :type "Actor Object Reference"))
  (cast `/Game/Blueprints/BP_EnemyRocketTurret` OtherActor
    (:`CastFailed`
      (cast `/Game/Blueprints/BP_PlayerCharacter` OtherActor
        (:`CastFailed`
          (`self.SpawnHitParticles` "/Game/Particles/RocketExlposion.RocketExlposion" (0.4 0.4 0.4))
          (`self.K2_DestroyActor` :!label _label))))))

(event `self.ReceiveTick`
  (params (DeltaSeconds :type "Float (single-precision)"))
  (bind _returnvalue (`self.K2_GetActorLocation`))
  (bind _returnvalue_2 (`self.K2_GetActorLocation` (`GameplayStatics.GetPlayerPawn` 0)))
  (`|ExecutionSequence`
    (:`then_0`
      (if true
        (`self.K2_SetActorLocationAndRotation` (`KismetMathLibrary.VInterpTo_Constant` _returnvalue _returnvalue_2 DeltaSeconds 500.0) (`KismetMathLibrary.RInterpTo` (`self.K2_GetActorRotation`) (`KismetMathLibrary.Conv_VectorToRotator` (- _returnvalue_2 _returnvalue)) DeltaSeconds 10.0))
        (`KismetSystemLibrary.Delay` 5.0)
        (`self.K2_DestroyActor`)))
    (:`then_1`
      (bind _asbp_player_character (cast `/Game/Blueprints/BP_PlayerCharacter` (stale `self.ReceiveActorBeginOverlap` OtherActor)))
      (if (`PrimitiveComponent.IsOverlappingActor` (`self.GetComponentByClass` _asbp_player_character "/Script/Engine.CapsuleComponent") self)
        (`PlayerCharacter.TakeDamage` _asbp_player_character (`self.ProjectileDamage`) (make `DamageEvent`) null null)
        (`self.SpawnHitParticles` "/Game/Particles/RocketExlposionClose.RocketExlposionClose" (0.1 0.1 0.1))
        (goto _label)))))

(fn `UserConstructionScript`)