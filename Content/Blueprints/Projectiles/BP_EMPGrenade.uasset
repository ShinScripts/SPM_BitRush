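; BP_EMPGrenade is a lobbed projectile grenade that damages player characters it overlaps.
; On BeginPlay it launches its cube with an impulse along negative forward plus lift, then destroys itself after a short delay.
; Overlapping a player applies ProjectileDamage and triggers a damage sound unless the grenade overlaps their deflector box; any other actor destroys it.
; Hit particle calls exist but are disconnected, and no EMP-specific effect is implemented.
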(event `self.ReceiveBeginPlay`
  (`PrimitiveComponent.AddImpulse` (`self.Cube`) (+ (* (`KismetMathLibrary.Conv_RotatorToVector` (`self.K2_GetActorRotation`)) (`KismetMathLibrary.Conv_DoubleToVector` -2000.0)) (0.0 0.0 300.0)) "None" false)
  (`KismetSystemLibrary.Delay` 3.0)
  (`self.K2_DestroyActor`))

(event `self.ReceiveActorBeginOverlap`
  (params (OtherActor :type "Actor Object Reference"))
  (bind _asbp_player_character (cast `/Game/Blueprints/BP_PlayerCharacter` OtherActor)
    (:`then`
      (bind _returnvalue (`PlayerCharacter.GetDeflectorBox` _asbp_player_character))
      (if (not (`PrimitiveComponent.IsOverlappingActor` _returnvalue self))
        (`PlayerCharacter.TakeDamage` _asbp_player_character (`self.ProjectileDamage`) (make `DamageEvent`) null null)
        (`AudioParameterControllerInterface.SetTriggerParameter` (`/Game/Blueprints/BP_PlayerCharacter.MSS_PickupDamageSounds` _asbp_player_character) "Damage")))
    (:`CastFailed`
      (`self.K2_DestroyActor`))))

(fn `UserConstructionScript`)