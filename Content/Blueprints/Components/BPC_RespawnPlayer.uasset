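; BPC_RespawnPlayer is an actor component that sends the player back to its start location when it hits the owning actor.
; On BeginPlay it binds to the owner's OnActorHit event.
; When the other actor casts to BP_PlayerCharacter, it moves the character to its stored StartLocation without sweep and zeroes its movement velocity.
; An unconnected level-reload path is left in the graph but never runs.
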(event `self.ReceiveBeginPlay`
  (add `Actor.OnActorHit` (`self.GetOwner`) (delegate `OnActorHit_Event`)))

(event `OnActorHit_Event`
  (params (SelfActor :type "Actor Object Reference") (OtherActor :type "Actor Object Reference") (NormalImpulse :type "Vector Structure") (Hit :type "HitResult Structure (by ref)"))
  (bind _asbp_player_character (cast `/Game/Blueprints/BP_PlayerCharacter` OtherActor))
  (`Actor.K2_SetActorLocation` _asbp_player_character (`/Game/Blueprints/BP_PlayerCharacter.StartLocation` _asbp_player_character) false false)
  (set `MovementComponent.Velocity` (0.0 0.0 0.0) (`Pawn.GetMovementComponent` _asbp_player_character)))