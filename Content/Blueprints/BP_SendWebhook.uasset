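; Trigger volume that reports level completion to a webhook when the player overlaps its Cube.
; On the first overlap by BP_PlayerCharacter, it builds a message with the current level name and a rounded time in seconds.
; PostTimeSinceStart selects either time since the trigger's creation or the player's remaining CurrentTime.
; The message is sent through SendWebhook on BP_BitRushGameMode.
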(event `self.Cube.OnComponentBeginOverlap`
  (params (OverlappedComponent :type "PrimitiveComponent Object Reference") (OtherActor :type "Actor Object Reference") (OtherComp :type "PrimitiveComponent Object Reference") (OtherBodyIndex :type Integer) (bFromSweep :type Boolean) (SweepResult :type "HitResult Structure (by ref)"))
  (bind _asbp_player_character (cast `/Game/Blueprints/BP_PlayerCharacter` OtherActor))
  (`/Engine/EditorBlueprintResources/StandardMacros.DoOnce` false
    (:`Completed`
      (bind _asbp_bit_rush_game_mode (cast `/Game/Blueprints/BP_BitRushGameMode` (`GameplayStatics.GetGameMode`)))
      (bind _returnvalue (`GameplayStatics.GetCurrentLevelName` true))
      (if (`self.PostTimeSinceStart`)
        (`Bit_RushGameModeBase.SendWebhook` _asbp_bit_rush_game_mode (`KismetStringLibrary.BuildString_Int` (`KismetStringLibrary.Concat_StrStr` "Level `" _returnvalue) "` finished in `" (`KismetMathLibrary.Round` (`self.GetGameTimeSinceCreation`)) "` seconds"))
        (else
          (`Bit_RushGameModeBase.SendWebhook` _asbp_bit_rush_game_mode (`KismetStringLibrary.BuildString_Int` (`KismetStringLibrary.Concat_StrStr` "Level `" _returnvalue) "` finished with `" (`KismetMathLibrary.Round` (`PlayerCharacter.CurrentTime` _asbp_player_character)) "` seconds remaining")))))))

(fn `UserConstructionScript`)