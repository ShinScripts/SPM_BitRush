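; Single sliding door actor that opens automatically when the player pawn comes near.
; BeginPlay caches the Left panel's world location as the closed position.
; Each Tick compares distance to player 0 against DistanceBeforeOpening and VInterps the panel toward the negated Offset or back to closed.
; The same check swaps Cube3's material between green and red emissive to indicate the state.
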(event `self.ReceiveBeginPlay`
  (set `self.StartLocation` (`SceneComponent.K2_GetComponentLocation` (`self.Left`))))

(event `self.ReceiveTick`
  (params (DeltaSeconds :type "Float (single-precision)"))
  (bind _left (`self.Left`))
  (bind _speed (`self.Speed`))
  (if (<= (`self.GetDistanceTo` (`GameplayStatics.GetPlayerPawn` 0)) (`self.DistanceBeforeOpening`))
    (`SceneComponent.K2_SetWorldLocation` (`self.Left`) (`KismetMathLibrary.VInterpTo` (`SceneComponent.K2_GetComponentLocation` (`self.Left`)) (+ (`self.StartLocation`) (* (`self.Offset`) -1.0)) DeltaSeconds _speed) false false)
    (`PrimitiveComponent.SetMaterial` (`self.Cube3`) 0 "/Game/Materials/Emissive_green.Emissive_green")
    (else
      (`SceneComponent.K2_SetWorldLocation` _left (`KismetMathLibrary.VInterpTo` (`SceneComponent.K2_GetComponentLocation` _left) (`self.StartLocation`) DeltaSeconds _speed) false false)
      (`PrimitiveComponent.SetMaterial` (`self.Cube3`) 0 "/Game/Materials/Emissive_Red.Emissive_Red"))))

(fn `UserConstructionScript`)