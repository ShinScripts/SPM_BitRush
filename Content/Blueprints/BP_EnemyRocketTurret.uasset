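; Rocket turret enemy that turns to face the player and fires while the player is within DistanceToPlayer.
; Each Tick it measures the distance to the player pawn and, when in range, snaps its rotation toward that pawn.
; A latent Delay on Tick paces the firing, and the range is checked again before calling Shoot, which is defined outside these graphs.
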(event `self.ReceiveTick`
  (params (DeltaSeconds :type "Float (single-precision)"))
  (bind _returnvalue (- (`self.K2_GetActorLocation` (`GameplayStatics.GetPlayerPawn` 0)) (`self.K2_GetActorLocation`)))
  (bind _returnvalue_2 (< (`KismetMathLibrary.Vector_Distance` _returnvalue) (`self.DistanceToPlayer`)))
  (if _returnvalue_2
    (`self.K2_SetActorRotation` (`KismetMathLibrary.Conv_VectorToRotator` _returnvalue))
    (`KismetSystemLibrary.Delay` (`self.Delay`))
    (if _returnvalue_2
      (`self.Shoot`))))

(fn `UserConstructionScript`)