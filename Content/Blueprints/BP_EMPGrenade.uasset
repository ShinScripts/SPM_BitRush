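; BP_EMPGrenade is an EMP grenade projectile that damages the player character on overlap.
; On BeginPlay it impulses its Cube along an axis derived from actor rotation, adding lift scaled by player distance, and self-destroys after a timed lifetime.
; Overlapping the player's deflector box suppresses both damage and explosion.
; Otherwise, overlaps play randomized sound and an explosion effect, damaging only the player, then destroy the actor after a delay.
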(event `self.ReceiveBeginPlay`
  (`PrimitiveComponent.AddImpulse` (`self.Cube`) (`KismetMathLibrary.MakeVector` (* (.x (`KismetMathLibrary.Conv_RotatorToVector` (`self.K2_GetActorRotation`))) -2000.0) (* (.y (`KismetMathLibrary.Conv_RotatorToVector` (`self.K2_GetActorRotation`))) -2000.0) (+ (* (.z (`KismetMathLibrary.Conv_RotatorToVector` (`self.K2_GetActorRotation`))) 1500.0) (+ (* (`KismetMathLibrary.VSize` (- (`self.K2_GetActorLocation` (`GameplayStatics.GetPlayerCharacter` 0)) (`self.K2_GetActorLocation`))) 0.3) 250.0))) "None" false)
  (`KismetSystemLibrary.Delay` 3.0)
  (`self.K2_DestroyActor`))

(event `self.ReceiveActorBeginOverlap`
  (params (OtherActor :type "Actor Object Reference"))
  (bind _returnvalue (`self.K2_GetActorLocation`))
  (bind _returnvalue_2 (`KismetMathLibrary.RandomFloatInRange` 0.95 1.05))
  (bind _asbp_player_character (cast `/Game/Blueprints/BP_PlayerCharacter` OtherActor)
    (:`then`
      (bind _returnvalue_3 (`PlayerCharacter.GetDeflectorBox` _asbp_player_character))
      (if (not (`PrimitiveComponent.IsOverlappingActor` _returnvalue_3 self))
        (`PlayerCharacter.TakeDamage` _asbp_player_character (`self.ProjectileDamage`) (make `DamageEvent`) null null)
        (`GameplayStatics.PlaySoundAtLocation` "/Game/Audio/Sounds/MSS_EmpProjectile_Sounds.MSS_EmpProjectile_Sounds" _returnvalue (struct) _returnvalue_2 _returnvalue_2 0.0 "/Game/Audio/TurretAttenuation.TurretAttenuation" null null null :!label _label)
        (`NiagaraFunctionLibrary.SpawnSystemAtLocation` "/Game/Particles/EMP_grenade_explosion.EMP_grenade_explosion" _returnvalue)
        (`KismetSystemLibrary.Delay` 1.0)
        (`self.K2_DestroyActor`)))
    (:`CastFailed`
      (goto _label))))

(fn `UserConstructionScript`)