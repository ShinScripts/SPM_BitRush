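; Mesh spawner tool Blueprint that builds an evenly spaced line of copies of one static mesh.
; The construction script adds the first mesh component without an offset, then loops up to Amount, accumulating the X, Y and Z offsets to place each further copy.
; All work happens in construction, with no active event graph logic.
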(fn `UserConstructionScript`
  (bind _returnvalue (`AddComponent|NODE_AddStaticMeshComponent-0`))
  (`StaticMeshComponent.SetStaticMesh` _returnvalue (`self.Static Mesh`))
  (for _ (range 2 (+ (`self.Amount`) 1))
    (bind _output_get (set `self.XCurrentAmount` (+ (`self.XOffset`) (`self.XCurrentAmount`))))
    (bind _output_get_2 (set `self.YCurrentAmount` (+ (`self.YOffset`) (`self.YCurrentAmount`))))
    (bind _output_get_3 (set `self.ZCurrentAmount` (+ (`self.ZOffset`) (`self.ZCurrentAmount`))))
    (bind _returnvalue_2 (`AddComponent|NODE_AddStaticMeshComponent-1` :`RelativeTransform` (`KismetMathLibrary.MakeTransform` (`KismetMathLibrary.MakeVector` _output_get _output_get_2 _output_get_3))))
    (`StaticMeshComponent.SetStaticMesh` _returnvalue_2 (`self.Static Mesh`))))