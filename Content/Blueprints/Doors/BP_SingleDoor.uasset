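; Single sliding door actor that opens automatically when the player pawn comes within a set distance and closes when it leaves.
; Tick interpolates the Left component between its starting position and an offset using VInterpTo, switching an indicator material between green and red.
; Two DoOnce nodes that reset each other play a positional door sound once per open or close, with randomized volume and pitch.
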(event `self.ReceiveBeginPlay`
  (set `self.StartLocation` (`SceneComponent.K2_GetComponentLocation` (`self.Left`))))

(event `self.ReceiveTick`
  (params (DeltaSeconds :type "Float (single-precision)"))
  (bind _returnvalue (`KismetMathLibrary.RandomFloatInRange` 0.8 1.2))
  (bind _returnvalue_2 (`KismetMathLibrary.RandomFloatInRange` 0.8 1.2))
  (bind _left (`self.Left`))
  (bind _speed (`self.Speed`))
  (if (<= (`self.GetDistanceTo` (`GameplayStatics.GetPlayerPawn` 0)) (`self.DistanceBeforeOpening`))
    (`SceneComponent.K2_SetWorldLocation` (`self.Left`) (`KismetMathLibrary.VInterpTo` (`SceneComponent.K2_GetComponentLocation` (`self.Left`)) (+ (`self.StartLocation`) (* (`self.Offset`) -1.0)) DeltaSeconds _speed) false false)
    (`PrimitiveComponent.SetMaterial` (`self.Cube3`) 0 "/Game/Materials/Door_green.Door_green")
    (`/Engine/EditorBlueprintResources/StandardMacros.DoOnce` false :!label _label
      (:`Completed`
        (`GameplayStatics.PlaySoundAtLocation` "/Game/Audio/Sounds/Other/Door1.Door1" (`self.K2_GetActorLocation`) (struct) _returnvalue_2 _returnvalue_2 0.0 "/Game/Audio/TurretAttenuation.TurretAttenuation" null null null)
        (goto _label_2 :!via `Reset`)))
    (else
      (`SceneComponent.K2_SetWorldLocation` _left (`KismetMathLibrary.VInterpTo` (`SceneComponent.K2_GetComponentLocation` _left) (`self.StartLocation`) DeltaSeconds _speed) false false)
      (`PrimitiveComponent.SetMaterial` (`self.Cube3`) 0 "/Game/Materials/Door_red.Door_red")
      (`/Engine/EditorBlueprintResources/StandardMacros.DoOnce` true :!label _label_2
        (:`Completed`
          (`GameplayStatics.PlaySoundAtLocation` "/Game/Audio/Sounds/Other/Door1.Door1" (`self.K2_GetActorLocation`) (struct) _returnvalue _returnvalue 0.0 "/Game/Audio/TurretAttenuation.TurretAttenuation" null null null)
          (goto _label :!via `Reset`))))))

(fn `UserConstructionScript`)