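; Single door that opens once its referenced FuseBox is no longer valid, for example after being destroyed.
; BeginPlay stores the Left component's start location, and Tick polls the FuseBox reference.
; While it is invalid, Tick interpolates Left toward the start minus Offset at Speed and sets Cube3's material to green.
; A DoOnce plays the door sound a single time with randomized volume and pitch.
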(event `self.ReceiveBeginPlay`
  (set `self.StartLocation` (`SceneComponent.K2_GetComponentLocation` (`self.Left`))))

(event `self.ReceiveTick`
  (params (DeltaSeconds :type "Float (single-precision)"))
  (bind _returnvalue (`KismetMathLibrary.RandomFloatInRange` 0.8 1.2))
  (if (not (`KismetSystemLibrary.IsValid` (`self.FuseBox`)))
    (`SceneComponent.K2_SetWorldLocation` (`self.Left`) (`KismetMathLibrary.VInterpTo` (`SceneComponent.K2_GetComponentLocation` (`self.Left`)) (+ (`self.StartLocation`) (* (`self.Offset`) -1.0)) DeltaSeconds (`self.Speed`)) false false)
    (`PrimitiveComponent.SetMaterial` (`self.Cube3`) 0 "/Game/Materials/Door_green.Door_green")
    (`/Engine/EditorBlueprintResources/StandardMacros.DoOnce` false
      (:`Completed`
        (`GameplayStatics.PlaySoundAtLocation` "/Game/Audio/Sounds/Other/Door1.Door1" (`self.K2_GetActorLocation`) (struct) _returnvalue _returnvalue 0.0 "/Game/Audio/TurretAttenuation.TurretAttenuation" null null null)))))

(fn `UserConstructionScript`)