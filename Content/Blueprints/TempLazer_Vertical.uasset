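; TempLazer_Vertical is a temporary vertical laser hazard that reloads the current level when its Cylinder component registers a hit.
; On BeginPlay it runs one Visibility trace from LineTranceStart along that component's up vector for Range units, with persistent debug drawing.
; It teleports the MSSLvlLaserbeam component to the midpoint between trace start and hit location, without rescaling it.
; The trace never updates after BeginPlay.
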(event `self.Cylinder.OnComponentHit`
  (params (HitComponent :type "PrimitiveComponent Object Reference") (OtherActor :type "Actor Object Reference") (OtherComp :type "PrimitiveComponent Object Reference") (NormalImpulse :type "Vector Structure") (Hit :type "HitResult Structure (by ref)"))
  (bind _returnvalue (`GameplayStatics.GetCurrentLevelName` true))
  (`GameplayStatics.OpenLevel` (`KismetStringLibrary.Conv_StringToName` _returnvalue)))

(event `self.ReceiveBeginPlay`
  (bind _linetrancestart (`self.LineTranceStart`))
  (bind _returnvalue (`SceneComponent.K2_GetComponentLocation` (`self.LineTranceStart`)))
  (bind _returnvalue_2 (`SceneComponent.K2_GetComponentLocation` _linetrancestart))
  (bind _outhit (`KismetSystemLibrary.LineTraceSingle` :`Start` _returnvalue_2 :`End` (+ _returnvalue_2 (* (`SceneComponent.GetUpVector` _linetrancestart) (`self.Range`))) :`TraceChannel` "TraceTypeQuery1" :`DrawDebugType` "Persistent" :`TraceColor` (struct :`R` 0.197228 :`G` 0.352879 :`B` 1.0 :`A` 1.0) :`DrawTime` 1.0))
  (`SceneComponent.K2_SetWorldLocation` (`self.MSS_LvlLaserbeam`) (- _returnvalue (/ (- _returnvalue (`.Location` (`GameplayStatics.BreakHitResult` _outhit))) (2.0 2.0 2.0))) false true))

(fn `UserConstructionScript`)