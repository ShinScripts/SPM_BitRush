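; BP_HintActor is a tutorial hint marker that plays a one-time attenuated sound when the player gets near and has line of sight.
; Tick checks horizontal distance and sight, with a name check giving BP_HintActor6 a longer range, then a short Delay leads into a DoOnce.
; The sound's pitch comes from the player's GuidePitch, which is nudged up afterwards so successive hints sound higher.
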(event `self.ReceiveBeginPlay`
  (bind _asbp_player_character (cast `/Game/Blueprints/BP_PlayerCharacter` (`GameplayStatics.GetPlayerCharacter` 0)))
  (set `self.BP_PlayerCharacter` _asbp_player_character))

(event `self.ReceiveTick`
  (params (DeltaSeconds :type "Float (single-precision)"))
  (bind _bp_playercharacter (`self.BP_PlayerCharacter`))
  (bind _returnvalue (`Controller.LineOfSightTo` (`GameplayStatics.GetPlayerController` 0) self (0.0 0.0 0.0) false))
  (bind _returnvalue_2 (`self.GetHorizontalDistanceTo` _bp_playercharacter))
  (set `self.TextGuidePitch` (`/Game/Blueprints/BP_PlayerCharacter.GuidePitch` _bp_playercharacter))
  (if (or (and (< _returnvalue_2 1400.0) _returnvalue) (and (< _returnvalue_2 2100.0) _returnvalue (== (`KismetSystemLibrary.GetDisplayName` self) "BP_HintActor6")))
    (`KismetSystemLibrary.Delay` 0.2)
    (`/Engine/EditorBlueprintResources/StandardMacros.DoOnce` false
      (:`Completed`
        (`GameplayStatics.PlaySoundAtLocation` "/Game/Audio/Sounds/Other/NewTutorialText.NewTutorialText" (`self.K2_GetActorLocation`) (struct) (`KismetMathLibrary.RandomFloatInRange` 0.9 1.1) (`self.TextGuidePitch`) 0.0 "/Game/Audio/GuideSoundAttenuation.GuideSoundAttenuation" null null null)
        (`KismetSystemLibrary.Delay` 1.0)
        (set `/Game/Blueprints/BP_PlayerCharacter.GuidePitch` (+ (`self.TextGuidePitch`) 0.05) (`self.BP_PlayerCharacter`))))))

(fn `UserConstructionScript`)