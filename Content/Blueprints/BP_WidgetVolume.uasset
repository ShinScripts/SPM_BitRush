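; BP_WidgetVolume is a trigger volume that shows and hides hint widgets as the player character enters and leaves it.
; On BeginPlay it toggles the widget of each BP_HintActor in its Widgets array, flipping the starting visibility.
; Begin and end overlaps with BP_PlayerCharacter toggle them again, guarded by an IsVisible flag.
; Visibility is relative, so results depend on each widget's initial state.
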(event `self.ReceiveBeginPlay`
  (for _array_element (`self.Widgets`)
    (bind _asbp_hint_actor (cast `/Game/Blueprints/BP_HintActor` _array_element))
    (`SceneComponent.ToggleVisibility` (`/Game/Blueprints/BP_HintActor.Widget` _asbp_hint_actor) false)))

(event `self.Volume.OnComponentBeginOverlap`
  (params (OverlappedComponent :type "PrimitiveComponent Object Reference") (OtherActor :type "Actor Object Reference") (OtherComp :type "PrimitiveComponent Object Reference") (OtherBodyIndex :type Integer) (bFromSweep :type Boolean) (SweepResult :type "HitResult Structure (by ref)"))
  (cast `/Game/Blueprints/BP_PlayerCharacter` OtherActor)
  (if (not (`self.IsVisible`))
    (for _array_element (`self.Widgets`)
      (bind _asbp_hint_actor (cast `/Game/Blueprints/BP_HintActor` _array_element))
      (`SceneComponent.ToggleVisibility` (`/Game/Blueprints/BP_HintActor.Widget` _asbp_hint_actor) false))
    (set `self.IsVisible` true)))

(event `self.Volume.OnComponentEndOverlap`
  (params (OverlappedComponent :type "PrimitiveComponent Object Reference") (OtherActor :type "Actor Object Reference") (OtherComp :type "PrimitiveComponent Object Reference") (OtherBodyIndex :type Integer))
  (cast `/Game/Blueprints/BP_PlayerCharacter` OtherActor)
  (if (`self.IsVisible`)
    (for _array_element (`self.Widgets`)
      (bind _asbp_hint_actor (cast `/Game/Blueprints/BP_HintActor` _array_element))
      (`SceneComponent.ToggleVisibility` (`/Game/Blueprints/BP_HintActor.Widget` _asbp_hint_actor) false))
    (set `self.IsVisible` false)))

(fn `UserConstructionScript`)