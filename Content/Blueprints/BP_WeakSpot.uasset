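; BP_WeakSpot is a destructible weak spot that shuts down linked turrets: DestroyTurrets destroys every actor in its Actors array, then itself.
; Tick triggers the MSSCablebox "Play" audio once, when the player controller has line of sight or the player is within set horizontal and vertical distances.
; On destruction it plays a turning-off sound at its location.
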(event `self.ReceiveTick`
  (params (DeltaSeconds :type "Float (single-precision)"))
  (bind _returnvalue (`GameplayStatics.GetPlayerCharacter` 0))
  (`|ExecutionSequence`
    (:`then_1`
      (if (or (`Controller.LineOfSightTo` (`GameplayStatics.GetPlayerController` 0) self (0.0 0.0 0.0) false) (and (< (`self.GetHorizontalDistanceTo` _returnvalue) 3000.0) (< (`self.GetVerticalDistanceTo` _returnvalue) 750.0)))
        (`/Engine/EditorBlueprintResources/StandardMacros.DoOnce` false
          (:`Completed`
            (`AudioParameterControllerInterface.SetTriggerParameter` (`self.MSS_Cablebox`) "Play")))))))

(event `self.ReceiveDestroyed`
  (`GameplayStatics.PlaySoundAtLocation` "/Game/Audio/Sounds/Enemy_Obstacles/PH_TurningOff.PH_TurningOff" (`self.K2_GetActorLocation`) (struct) 1.0 1.0 0.0 null null null null))

(fn `DestroyTurrets`
  (for _array_element (`self.Actors`)
    (`self.K2_DestroyActor` _array_element))
  (`self.K2_DestroyActor`))

(fn `UserConstructionScript`)