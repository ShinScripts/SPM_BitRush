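; Player character that wall-runs along surfaces to either side, jumps off them and fires a debug hitscan shot.
; While falling, side line traces each Tick set forward velocity, zero gravity and lock vertical movement via plane constraint; a miss calls OffWall to restore both.
; Jump launches away from the wall, briefly suppressing wall-run.
; Left mouse traces from the camera and prints the hit component; damage logic is unconnected.
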(event `Key|LeftMouseButton`
  (params (Key :type "Key Structure"))
  (:`Pressed`
    (`self.FireProjectile`)))

(event `self.ReceiveBeginPlay`
  (`MovementComponent.SetPlaneConstraintEnabled` (`self.CharacterMovement`) true))

(event `self.ReceiveTick`
  (params (DeltaSeconds :type "Float (single-precision)"))
  (`self.RightWallRun`)
  (`self.LeftWallRun`))

(event `InputAction|Jump`
  (params (Key :type "Key Structure"))
  (bind (_returnvalue_x _returnvalue_y) (`KismetMathLibrary.BreakVector` (select `bool` (`self.OnRightSide`) :`false` (* (`self.GetActorRightVector`) 900.0) :`true` (* (`self.GetActorRightVector`) -900.0))))
  (:`Pressed`
    (if (or (`self.RightSide?`) (`self.LeftSide?`))
      (set `self.IsJumpingOffWall` true)
      (`self.LaunchCharacter` (`KismetMathLibrary.MakeVector` _returnvalue_x _returnvalue_y 450.0) false true)
      (`KismetSystemLibrary.Delay` 0.2)
      (set `self.IsJumpingOffWall` false)
      (else
        (`self.Jump`)))))

(fn `FireProjectile`
  (bind _camera (`self.Camera`))
  (bind _returnvalue (`SceneComponent.K2_GetComponentLocation` _camera))
  (bind (_outhit _returnvalue_2) (`KismetSystemLibrary.LineTraceSingle` :`Start` _returnvalue :`End` (+ _returnvalue (* (`SceneComponent.GetForwardVector` _camera) (`self.GunRange`))) :`TraceChannel` "TraceTypeQuery1" :`DrawDebugType` "ForDuration" :`DrawTime` 1.0))
  (if _returnvalue_2
    (`KismetSystemLibrary.PrintString` (`KismetSystemLibrary.GetDisplayName` (`.HitComponent` (`GameplayStatics.BreakHitResult` _outhit))))))

(fn `LeftWallRun`
  (bind _returnvalue (`self.K2_GetActorLocation`))
  (bind _charactermovement (`self.CharacterMovement`))
  (bind (_returnvalue_x _returnvalue_y) (`KismetMathLibrary.BreakVector` (* (`self.GetActorForwardVector`) 500.0)))
  (if (`NavMovementComponent.IsFalling` (`self.CharacterMovement`))
    (bind (_outhit _returnvalue_2) (`KismetSystemLibrary.LineTraceSingle` :`Start` _returnvalue :`End` (+ _returnvalue (* (`self.GetActorRightVector`) (* (`self.LineTraceLength`) -1.0))) :`TraceChannel` "TraceTypeQuery1" :`DrawDebugType` "ForDuration"))
    (if _returnvalue_2
      (set `self.LeftSide?` true)
      (set `self.OnRightSide` false)
      (if (not (`self.IsJumpingOffWall`))
        (set `MovementComponent.Velocity` (`KismetMathLibrary.MakeVector` _returnvalue_x _returnvalue_y) _charactermovement)
        (set `CharacterMovementComponent.GravityScale` 0.0 _charactermovement)
        (`MovementComponent.SetPlaneConstraintNormal` _charactermovement (0.0 0.0 1.0)))
      (else
        (set `self.LeftSide?` false)
        (`self.OffWall`)))))

(fn `OffWall`
  (bind _charactermovement (`self.CharacterMovement`))
  (set `CharacterMovementComponent.GravityScale` 1.0 _charactermovement)
  (`MovementComponent.SetPlaneConstraintNormal` _charactermovement (0.0 0.0 0.0)))

(fn `RightWallRun`
  (bind _returnvalue (`self.K2_GetActorLocation`))
  (bind _charactermovement (`self.CharacterMovement`))
  (bind (_returnvalue_x _returnvalue_y) (`KismetMathLibrary.BreakVector` (* (`self.GetActorForwardVector`) 500.0)))
  (if (`NavMovementComponent.IsFalling` (`self.CharacterMovement`))
    (bind (_outhit _returnvalue_2) (`KismetSystemLibrary.LineTraceSingle` :`Start` _returnvalue :`End` (+ _returnvalue (* (`self.GetActorRightVector`) (`self.LineTraceLength`))) :`TraceChannel` "TraceTypeQuery1" :`DrawDebugType` "ForDuration"))
    (if _returnvalue_2
      (bind _output_get (set `self.RightSide?` true))
      (set `self.OnRightSide` _output_get)
      (if (not (`self.IsJumpingOffWall`))
        (set `MovementComponent.Velocity` (`KismetMathLibrary.MakeVector` _returnvalue_x _returnvalue_y) _charactermovement)
        (set `CharacterMovementComponent.GravityScale` 0.0 _charactermovement)
        (`MovementComponent.SetPlaneConstraintNormal` _charactermovement (0.0 0.0 1.0)))
      (else
        (set `self.RightSide?` false)
        (`self.OffWall`)))))

(fn `UserConstructionScript`)