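; BP_EnemyLaserTurret is an enemy turret that turns to track the player pawn, with no firing logic in this graph.
; Each tick it leads the target by adding a fraction of the pawn's velocity to its location.
; When that predicted point is in range, the whole actor rotates toward it at a constant rate through RInterpToConstant.
; A trailing Delay has nothing after it, and the construction script is empty.
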(event `self.ReceiveTick`
  (params (DeltaSeconds :type "Float (single-precision)"))
  (bind _returnvalue (`GameplayStatics.GetPlayerPawn` 0))
  (bind _returnvalue_2 (- (+ (* (`self.GetVelocity` _returnvalue) (0.2 0.2 0.2)) (`self.K2_GetActorLocation` _returnvalue)) (`self.K2_GetActorLocation`)))
  (if (< (`KismetMathLibrary.Vector_Distance` _returnvalue_2) 10000.0)
    (`self.K2_SetActorRotation` (`KismetMathLibrary.RInterpTo_Constant` (`self.K2_GetActorRotation`) (`KismetMathLibrary.Conv_VectorToRotator` _returnvalue_2) DeltaSeconds 100.0))
    (`KismetSystemLibrary.Delay` 5.0)))

(fn `UserConstructionScript`)